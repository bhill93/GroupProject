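; Exploding barrel actor that detonates when its Hit event fires, then destroys itself.
; Hit spawns two explosion emitters and force feedback at the hit location, with the explosion sound played at world origin.
; It also starts a camera shake on the first player and fires the ExplosionForce impulse.
; A brief global time dilation gives a slow-motion beat before normal speed is restored and the actor is destroyed.
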(event Collision|EventHit
  (params (MyComp :type Primitive%20Component%20Object%20Reference) (Other :type Actor%20Object%20Reference) (OtherComp :type Primitive%20Component%20Object%20Reference) (bSelfMoved :type Boolean) (HitLocation :type Vector :default "0, 0, 0") (HitNormal :type Vector :default "0, 0, 0") (NormalImpulse :type Vector :default "0, 0, 0") (Hit :type Hit%20Result%20Structure%20%28by%20ref%29))
  (Collision|SetCollisionEnabled (Variables|Default|GetBarrel) "QueryAndPhysics")
  (Development|PrintString "Hit Detected")
  (Effects|SpawnEmitteratLocation "/Engine/Tutorial/SubEditors/TutorialAssets/TutorialParticleSystem.TutorialParticleSystem" HitLocation "0, 0, 0" "5.000000,5.000000,5.000000")
  (Audio|PlaySoundatLocation "/Game/Explosion.Explosion" "0, 0, 0" "0, 0, 0" 1.0 1.0 0.0 0 0 0 0)
  (ForceFeedback|SpawnForceFeedbackatLocation "/Game/FFE_Explosion.FFE_Explosion" HitLocation "0, 0, 0" false 1.0 0.0 0)
  (Effects|SpawnEmitteratLocation "/Engine/Tutorial/SubEditors/TutorialAssets/TutorialParticleSystem.TutorialParticleSystem" HitLocation)
  (Class|LegacyCameraShake|StartLegacyCameraShake (Game|GetPlayerCameraManager 0) "/Game/CameraShake/LCS_Explosion.LCS_Explosion_C" 1.0 "World" "0, 0, 0")
  (Class|RadialForceComponent|FireImpulse (Variables|Default|GetExplosionForce))
  (Utilities|Time|SetGlobalTimeDilation 0.3)
  (Utilities|FlowControl|Delay 0.15)
  (Utilities|Time|SetGlobalTimeDilation 1.0)
  (Actor|DestroyActor))

(fn ConstructionScript)